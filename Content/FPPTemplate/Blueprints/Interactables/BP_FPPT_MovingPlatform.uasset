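; Power-driven moving platform that travels along an editable spline while active.
; A gated Tick advances distance along the spline, with movement type choosing ping-pong, closed loop, wrap to start or stop at end.
; Inherited power-update events open or close the gate and toggle the movement sound.
; Construction colors the spline by power type, applies point types and previews the platform position.
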(event Custom|Update%20Spline
  (bind _power_type (Variables|Default|GetPower%20Type))
  (bind _type_colors (CallFunction|GetPowerTypeColors _power_type))
  (bind (_basecolor _emissivecolor) (Utilities|Struct|BreakStruct_FPPT_Colors _type_colors))
  ;[1 1 1] Update Spline Colors and Types
  (Class|SplineComponent|SetUnselectedSplineSegmentColor (Variables|Default|GetSpline) (Math|Conversions|ToLinearColor(Color) _basecolor))
  (Class|SplineComponent|SetSelectedSplineSegmentColor (Variables|Default|GetSpline) (Math|Conversions|ToLinearColor(Color) _emissivecolor))
  (Spline|SetClosedLoop (Variables|Default|GetSpline) (Utilities|Enum|Equal(Enum) (Variables|Default|GetMovement%20Type) "NewEnumerator2") true)
  (for _index (range 0 (Spline|GetNumberOfSplinePoints (Variables|Default|GetSpline)))
    (Spline|SetSplinePointType (Variables|Default|GetSpline) _index (Variables|Default|GetSpline%20Type) true)))

(event Custom|Start%20Moving
  (Utilities|FlowControl|Gate (not (Variables|Default|GetActive))) ; enters at Open
)

(event Custom|Update%20Movement
  (params (Delta%20Seconds :type Float%20%28single-precision%29))
  (bind _spline (Variables|Default|GetSpline))
  (bind _movement_type (Variables|Default|GetMovement%20Type))
  (bind _movement_type_2 (Variables|Default|GetMovement%20Type))
  (bind _spline_2 (Variables|Default|GetSpline))
  (bind _movement_speed (Variables|Default|GetMovement%20Speed))
  (bind _returnvalue (Spline|GetSplineLength _spline_2))
  (bind _returnvalue_2 (* Delta%20Seconds _movement_speed))
  (if (< (Variables|Default|GetCurrent%20Position) 0.0)
    (Variables|Default|SetInverse false)
    (elif (> (Variables|Default|GetCurrent%20Position) _returnvalue)
      (Variables|Default|SetInverse true)))
  (bind _output_get (Variables|Default|SetCurrent%20Position (Math|Float|SelectFloat (+ (Math|Float|SelectFloat (Variables|Default|GetCurrent%20Position) (Math|Float|SelectFloat (- (Variables|Default|GetCurrent%20Position) _returnvalue) (Variables|Default|GetCurrent%20Position) (and (> (Variables|Default|GetCurrent%20Position) _returnvalue) (or (Utilities|Enum|Equal(Enum) _movement_type_2 "NewEnumerator2") (Utilities|Enum|Equal(Enum) _movement_type_2 "NewEnumerator3")))) (Utilities|Enum|Equal(Enum) (Variables|Default|GetMovement%20Type) "NewEnumerator1")) (Math|Float|SelectFloat (* _returnvalue_2 -1.0) _returnvalue_2 (and (Utilities|Enum|Equal(Enum) (Variables|Default|GetMovement%20Type) "NewEnumerator1") (Variables|Default|GetInverse)))) (Math|Float|Clamp(Float) (+ (Math|Float|SelectFloat (Variables|Default|GetCurrent%20Position) (Math|Float|SelectFloat (- (Variables|Default|GetCurrent%20Position) _returnvalue) (Variables|Default|GetCurrent%20Position) (and (> (Variables|Default|GetCurrent%20Position) _returnvalue) (or (Utilities|Enum|Equal(Enum) _movement_type_2 "NewEnumerator2") (Utilities|Enum|Equal(Enum) _movement_type_2 "NewEnumerator3")))) (Utilities|Enum|Equal(Enum) (Variables|Default|GetMovement%20Type) "NewEnumerator1")) (Math|Float|SelectFloat (* _returnvalue_2 -1.0) _returnvalue_2 (and (Utilities|Enum|Equal(Enum) (Variables|Default|GetMovement%20Type) "NewEnumerator1") (Variables|Default|GetInverse)))) 0.0 (Spline|GetSplineLength _spline)) (Math|Boolean|ORBoolean (Utilities|Enum|Equal(Enum) _movement_type "NewEnumerator2") (Utilities|Enum|Equal(Enum) _movement_type "NewEnumerator3") (Utilities|Enum|Equal(Enum) _movement_type "NewEnumerator1")))))
  (Transformation|SetRelativeLocation (Variables|Default|GetPlatform) (Spline|GetLocationatDistanceAlongSpline _spline _output_get "Local") false false))

(event Custom|Stop%20Moving
  (Utilities|FlowControl|Gate (not (Variables|Default|GetActive))) ; enters at Close
)

(event Custom|Update%20Movement%20Tick
  (params (Delta%20Seconds :type Float%20%28single-precision%29))
  (Utilities|FlowControl|Gate (not (Variables|Default|GetActive))
    (:Exit
      (CallFunction|UpdateMovement Delta%20Seconds))))

(event EventBeginPlay
  (|CallParentFunction)
  (Audio|Components|Audio|SetSound (Variables|Default|GetSoundMovingComponent) (Variables|Default|GetSoundMoving))
  (if (Variables|Default|GetActive)
    (Audio|Components|Audio|Play (Variables|Default|GetSoundMovingComponent) 0.0)))

(event Collision|EventActorBeginOverlap
  (params (OtherActor :type Actor%20Object%20Reference))
  (|CallParentFunction OtherActor) ; This node is disabled and will not be called.\nDrag off pins to build functionality.
)

(event EventTick
  (params (DeltaSeconds :type Float%20%28single-precision%29))
  (|CallParentFunction DeltaSeconds)
  (CallFunction|UpdateMovementTick DeltaSeconds))

(event EventSetupMaterialOwners
  (bind _main_power_material (Variables|Default|GetMain%20Power%20Material))
  (bind _staticmesh (Variables|Default|GetStaticMesh))
  (Rendering|Material|SetMaterial _staticmesh 0 _main_power_material)
  (Rendering|Material|SetMaterial _staticmesh 1 _main_power_material)
  (Rendering|Material|SetMaterial _staticmesh 2 _main_power_material)
  (Rendering|Material|SetMaterial _staticmesh 3 _main_power_material)
  (Rendering|Material|SetMaterial _staticmesh 7 _main_power_material))

(event EventRunConstructionScriptsNonGenerative
  (params (Forced :type Boolean))
  (|CallParentFunction Forced)
  (CallFunction|UpdateSpline))

(event EventOnUpdatePowerUpdate
  (params (Current%20Amount :type Float%20%28single-precision%29))
  (CallFunction|UpdatePositions Current%20Amount))

(event EventOnUpdatePowerFinished
  (params (Forced :type Boolean))
  (bind _soundmovingcomponent (Variables|Default|GetSoundMovingComponent))
  (CallFunction|UpdatePositions (Math|Conversions|ToFloat(Boolean) (Variables|Default|GetActive)))
  (if (Variables|Default|GetActive)
    (CallFunction|StartMoving)
    (Audio|Components|Audio|Play _soundmovingcomponent 0.0)
    (else
      (CallFunction|StopMoving)
      (Audio|Components|Audio|Stop _soundmovingcomponent))))

(fn ConstructionScript
  (|CallParentFunction)
  (CallFunction|UpdateMovement 0.0))

(fn UpdatePositions
  (params (Amount :type Float%20%28single-precision%29)))

(fn ResetSpline
  (bind _spline (Variables|Default|GetSpline))
  (Spline|ClearSplinePoints _spline false)
  (Spline|AddSplinePoint _spline (Math|Vector|MakeVector 0.0 0.0 0.0) "Local" false)
  (Spline|AddSplinePoint _spline (Math|Vector|MakeVector 0.0 2e+02 0.0) "Local" true))